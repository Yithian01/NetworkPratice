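; Lobby HUD Blueprint that creates and displays the WBP_Lobby widget.
; On BeginPlay it caches the lobby player controller and, in a following Sequence step, adds the widget to the viewport.
; GetLobbyUI lazily creates and caches the widget, and RefreshUI uses it to forward refresh calls to that widget.
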(event `self.ReceiveBeginPlay`
  (`|ExecutionSequence`
    (:`then_0`
      (bind _asbp_player_controller_lobby (cast `/Game/Blueprints/Lobby/BP_PlayerController_Lobby` (`GameplayStatics.GetPlayerController` 0)))
      (set `self.PlayerController_Ref` _asbp_player_controller_lobby))
    (:`then_1`
      (bind _lobbyui (`self.GetLobbyUI`))
      (`UserWidget.AddToViewport` _lobbyui 0))))

(fn `GetLobbyUI`
  (returns (LobbyUI :type "/Widget/Lobby/WBP_Lobby Object Reference"))
  (`/Engine/EditorBlueprintResources/StandardMacros.IsValid` (`self.LobbyUI`)
    (:`Is Valid`
      _)
    (:`Is Not Valid`
      (bind _returnvalue (`|CreateWidget` "/Widget/Lobby/WBP_Lobby.WBP_Lobby_C"))
      (set `self.LobbyUI` _returnvalue)))
  (return (`self.LobbyUI`)))

(fn `RefreshUI`
  (bind _lobbyui (`self.GetLobbyUI`))
  (`/Widget/Lobby/WBP_Lobby.RefreshUI` _lobbyui))

(fn `UserConstructionScript`)