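; Player controller for the lobby that runs in UI-only input mode with a visible mouse cursor.
; BeginPlay sets the input mode and cursor and prints a debug string.
; The S2C_UpdateUI event, named as a server-to-client call, refreshes the lobby HUD's UI, lazily casting and caching the BP_Hud_Lobby reference on first use.
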(event `self.ReceiveBeginPlay`
  (`WidgetBlueprintLibrary.SetInputMode_UIOnlyEx` self null)
  (set `self.bShowMouseCursor` true)
  (`KismetSystemLibrary.PrintString` "PC" true true (struct :`G` 0.66 :`B` 1.0 :`A` 1.0) 999.0))

(event `S2C_UpdateUI`
  (`/Engine/EditorBlueprintResources/StandardMacros.IsValid` (`self.Hud_Ref`)
    (:`Is Valid`
      _)
    (:`Is Not Valid`
      (bind _asbp_hud_lobby (cast `/Game/Blueprints/Lobby/BP_Hud_Lobby` (`self.GetHUD`)))
      (set `self.Hud_Ref` _asbp_hud_lobby)))
  (`/Game/Blueprints/Lobby/BP_Hud_Lobby.RefreshUI` (`self.Hud_Ref`)))

(fn `UserConstructionScript`)